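; Player character Blueprint that shows the height and radius of a pooled object, apparently a tree, that the player clicks on.
; BeginPlay creates a hidden Height_Radius_UI widget.
; Left click runs a debug-drawn visibility trace from the actor along control rotation.
; On a blocking hit, the HitItem index queries the first TreeSpawnManager's ActorPooler, and the widget displays the result in Game and UI input mode.
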(event EventBeginPlay
  (bind _returnvalue (UserInterface|CreateWidget "/Game/Widget/Height_Radius_UI.Height_Radius_UI_C" (Game|GetPlayerController 0)))
  (bind _output_get (Variables|Default|SetWidgetRefernce _returnvalue))
  (UserInterface|Viewport|AddtoViewport _output_get 0)
  (Widget|SetVisibility _output_get "Hidden"))

(event Collision|EventActorBeginOverlap
  (params (OtherActor :type Actor%20Object%20Reference)))

(event EventTick
  (params (DeltaSeconds :type Float%20%28single-precision%29)))

(event Input|MouseEvents|LeftMouseButton
  (params (Key :type Key%20Structure :default "None"))
  (bind _returnvalue (Transformation|GetActorLocation))
  (bind _widgetrefernce (Variables|Default|GetWidgetRefernce))
  ;[1 1 1] Code for display Height and Radius based on Line Trace
  (:Pressed
    (bind _outhit (Collision|LineTraceByChannel _returnvalue (+ _returnvalue (* (Math|Vector|GetForwardVector (Pawn|GetControlRotation (Pawn|GetController) :!class /Script/Engine.Controller)) 1e+04)) "TraceTypeQuery1" false 0 "ForDuration" true "(R=1.000000,G=0.000000,B=0.000000,A=1.000000)" "(R=0.000000,G=1.000000,B=0.000000,A=1.000000)" 2.0))
    (if (.bBlockingHit (Collision|BreakHitResult _outhit))
      (bind _outactors (Actor|GetAllActorsOfClass "/Script/TreeGeneration.TreeSpawnManager"))
      (bind _returnvalue_2 (Class|TreePoolingObject|GetPooledObjectDetails (Variables|/Script/TreeGeneration.TreeSpawnManager|GetActorPooler (Utilities|Array|Get(acopy) _outactors)) (.HitItem (Collision|BreakHitResult _outhit))))
      (Widget|SetVisibility _widgetrefernce "Visible")
      (Input|SetInputModeGameandUI (Game|GetPlayerController 0) _widgetrefernce "DoNotLock" true)
      (Default|DisplayHeightRadius _widgetrefernce (Utilities|Array|Get(acopy) _returnvalue_2 1) (Utilities|Array|Get(acopy) _returnvalue_2)))))

(fn ConstructionScript)